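; Enemy actor that chases the player, deals contact damage and drops a BP_Xp pickup when killed.
; Tick turns it toward the cached player and steps it forward by Speed each frame, without delta-time scaling or sweep.
; Sphere overlap damages the player, pushes the enemy back and briefly blocks further hits via a Hit flag.
; Overlapping actors tagged Gun are destroyed and subtract the player's DmgGun from its HP before the death check.
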(event `self.ReceiveBeginPlay`
  (`|ExecutionSequence`
    (:`then_0`
      ;[1 1 1] Cast Player
      (bind _asbp_joueur (cast `/Game/Characters/BP_Joueur` (`GameplayStatics.GetPlayerCharacter` 0)))
      (set `self.As BP Joueur` _asbp_joueur))))

(event `self.ReceiveTick`
  (params (DeltaSeconds :type "Float (single-precision)"))
  ;[1 1 1] Move to player
  (`self.K2_SetActorRotation` (`KismetMathLibrary.FindLookAtRotation` (`self.K2_GetActorLocation`) (`self.K2_GetActorLocation` (`self.As BP Joueur`))))
  (`self.K2_SetActorRelativeLocation` (+ (`self.K2_GetActorLocation`) (* (`self.GetActorForwardVector`) (`self.Speed`)))))

(event `Death?`
  (bind _returnvalue_location (`KismetMathLibrary.BreakTransform` (`self.GetTransform`)))
  ;[1 1 1] Death
  (if (<= (`self.HP`) 0.0)
    (`|SpawnActorFromClass` "/Game/BP/BP_Xp.BP_Xp_C" (`KismetMathLibrary.MakeTransform` _returnvalue_location) "Undefined" "MultiplyWithRoot" null null)
    (`self.K2_DestroyActor`)
    (`AddComponent|NODE_AddParticleSystemComponent-1`)))

(event `self.Sphere.OnComponentBeginOverlap`
  (params (OverlappedComponent :type "PrimitiveComponent Object Reference") (OtherActor :type "Actor Object Reference") (OtherComp :type "PrimitiveComponent Object Reference") (OtherBodyIndex :type Integer) (bFromSweep :type Boolean) (SweepResult :type "HitResult Structure (by ref)"))
  ;[1 1 1] Colision Player
  (if (== OtherActor (`self.As BP Joueur`))
    (if (not (`self.Hit?`))
      (set `self.Hit?` true)
      (bind _asbp_joueur (cast `/Game/Characters/BP_Joueur` (`GameplayStatics.GetPlayerCharacter` 0)))
      (bind _hp (`/Game/Characters/BP_Joueur.HP` _asbp_joueur))
      (set `/Game/Characters/BP_Joueur.HP` (- _hp (`self.Dmg`)) _asbp_joueur)
      (`KismetSystemLibrary.PrintString` (`KismetStringLibrary.Conv_IntToString` _hp))
      (if (<= _hp 0)
        (`/Game/Characters/BP_Joueur.Death` _asbp_joueur))
      (`self.K2_SetActorRelativeLocation` (- (`self.K2_GetActorLocation`) (* (`self.GetActorForwardVector`) (100.0 100.0 100.0))))
      (`KismetSystemLibrary.Delay` 0.5)
      (set `self.Hit?` false))
    (elif (`self.ActorHasTag` OtherActor "Gun")
      ;[1 1 1] Gun
      (bind _asbp_joueur_2 (cast `/Game/Characters/BP_Joueur` (`GameplayStatics.GetPlayerCharacter` 0)))
      (set `self.HP` (- (`self.HP`) (`/Game/Characters/BP_Joueur.DmgGun` _asbp_joueur_2)))
      (`self.K2_DestroyActor` OtherActor)
      (`self.Death?`))))

(fn `UserConstructionScript`)