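; BP_Joueur is the player character, which moves on input, faces the mouse cursor and fires automatically.
; Each Tick a cursor line trace sets the mesh yaw, while a looping delay started at BeginPlay spawns BP_GunShot from the Gunshot component.
; XP pickups raise the level at a threshold, opening the Wdg_LvlUp widget and pausing the game.
; Death only adds a particle component, and StatAugmente only prints its value.
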(event `self.ReceiveTick`
  (params (DeltaSeconds :type "Float (single-precision)"))
  (bind (_worldlocation _worlddirection) (`PlayerController.DeprojectMousePositionToWorld` (`GameplayStatics.GetPlayerController` 0)))
  ;[1 1 1] Rotation
  (bind _outhit (`KismetSystemLibrary.LineTraceSingle` _worldlocation (+ _worldlocation (* _worlddirection (+ (`SpringArmComponent.TargetArmLength` (`self.SpringArm`)) 2400.0))) "TraceTypeQuery1"))
  (bind _output_get (set `self.Out Hit Location` (`.Location` (`GameplayStatics.BreakHitResult` _outhit))))
  (bind (_returnvalue_roll _returnvalue_pitch _returnvalue_yaw) (`KismetMathLibrary.BreakRotator` (`KismetMathLibrary.FindLookAtRotation` (`self.K2_GetActorLocation`) _output_get)))
  (`SceneComponent.K2_SetWorldRotation` (`self.Mesh`) (`KismetMathLibrary.MakeRotator` _returnvalue_roll 0.0 _returnvalue_yaw) false false))

(event `self.ReceiveBeginPlay`
  (`self.Gun`))

(event `EnhancedInput|/Game/Characters/IA_Movement`
  (params (ActionValue :type "Vector2D Structure") (ElapsedSeconds :type "Float (double-precision)") (TriggeredSeconds :type "Float (double-precision)") (InputAction :type "InputAction Object Reference" :default "/Game/Characters/IA_Movement.IA_Movement"))
  (bind (_returnvalue_roll _returnvalue_pitch _returnvalue_yaw) (`KismetMathLibrary.BreakRotator` (`self.GetControlRotation`)))
  (bind _returnvalue (`KismetMathLibrary.MakeRotator` 0.0 0.0 _returnvalue_yaw))
  ;[1 1 1] Movement
  (:`Triggered`
    (`|ExecutionSequence`
      (:`then_0`
        (`self.AddMovementInput` (`KismetMathLibrary.GetForwardVector` _returnvalue) ActionValue_Y))
      (:`then_1`
        (`self.AddMovementInput` (`KismetMathLibrary.GetRightVector` _returnvalue) ActionValue_X)))))

(event `Death`
  ;[1 1 1] Mort
  (`AddComponent|NODE_AddParticleSystemComponent-1`))

(event `PickupXP`
  ;[1 1 1] XP
  (set `self.XP` (+ (`self.XP`) 1.0))
  (if (>= (`self.XP`) (`self.XpToNextLvl`))
    (set `self.Lvl` (+ (`self.Lvl`) 1))
    (set `self.XP` 0.0)
    (`self.LvlUp`)))

(event `Gun`
  (bind (_returnvalue_location _returnvalue_rotation) (`KismetMathLibrary.BreakTransform` (`SceneComponent.K2_GetComponentToWorld` (`self.Gunshot`))))
  ;[1 1 1] Gun
  (`KismetSystemLibrary.Delay` (`self.CadenceGun`) :!label _label)
  (`|SpawnActorFromClass` "/Game/Weapon/BP_GunShot.BP_GunShot_C" (`KismetMathLibrary.MakeTransform` _returnvalue_location _returnvalue_rotation) "Undefined" "MultiplyWithRoot" null null)
  (goto _label))

(event `LvlUp`
  ;[1 1 1] LvlUpStats
  (bind _returnvalue (`|CreateWidget` "/Game/Characters/Wdg_LvlUp.Wdg_LvlUp_C"))
  (`UserWidget.AddToViewport` _returnvalue 0)
  (`GameplayStatics.SetGamePaused` true))

(event `StatAugmente`
  (params (Augmente :type Integer))
  ;[1 1 1] LvlUpStats
  (`KismetSystemLibrary.PrintString` (`KismetStringLibrary.Conv_IntToString` Augmente)))

(fn `UserConstructionScript`)