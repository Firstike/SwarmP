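; BP_Spawner is an actor that spawns an enemy at a random direction around the player when its SpawnEnemy event is called.
; The event snaps the spawner to the BP_Joueur player's location and gives it a random yaw, so its SpawnPoint component determines where the actor appears.
; It then activates the NiaSpawn effect component, with no logic on BeginPlay or Tick.
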(event `self.ReceiveBeginPlay`)

(event `SpawnEnemy`
  ;[1 1 1] TriggerSpawn
  (bind _asbp_joueur (cast `/Game/Characters/BP_Joueur` (`GameplayStatics.GetPlayerCharacter` 0)))
  (`self.K2_SetActorRotation` (`KismetMathLibrary.MakeRotator` 0.0 0.0 (`KismetMathLibrary.RandomFloatInRange` 0.0 359.0)))
  (bind (_returnvalue_x _returnvalue_y _returnvalue_z) (`KismetMathLibrary.BreakVector` (`self.K2_GetActorLocation` _asbp_joueur)))
  (`self.K2_SetActorLocation` (`KismetMathLibrary.MakeVector` _returnvalue_x _returnvalue_y _returnvalue_z))
  (`|SpawnActorFromClass` "/Game/Enemi/BP_Enemy.BP_Enemy_C" (`SceneComponent.K2_GetComponentToWorld` (`self.SpawnPoint`)) "Undefined" "MultiplyWithRoot" null null)
  (`ActorComponent.Activate` (`self.Nia_Spawn`) false))

(fn `UserConstructionScript`)