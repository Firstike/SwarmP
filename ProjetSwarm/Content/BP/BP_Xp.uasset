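; BP_Xp is an experience pickup that the player character collects by overlap.
; On BeginPlay it sizes its Sphere1 collision from the XpRadius variable on BP_Joueur.
; When that player enters the sphere, it calls PickupXP on the player and destroys itself.
; The radius is read only once, at spawn, and other overlapping actors are ignored.
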(event `self.ReceiveBeginPlay`
  (bind _asbp_joueur (cast `/Game/Characters/BP_Joueur` (`GameplayStatics.GetPlayerCharacter` 0)))
  (`SphereComponent.SetSphereRadius` (`self.Sphere1`) (`/Game/Characters/BP_Joueur.XpRadius` _asbp_joueur) true))

(event `self.Sphere1.OnComponentBeginOverlap`
  (params (OverlappedComponent :type "PrimitiveComponent Object Reference") (OtherActor :type "Actor Object Reference") (OtherComp :type "PrimitiveComponent Object Reference") (OtherBodyIndex :type Integer) (bFromSweep :type Boolean) (SweepResult :type "HitResult Structure (by ref)"))
  (bind _asbp_joueur (cast `/Game/Characters/BP_Joueur` (`GameplayStatics.GetPlayerCharacter` 0)))
  (if (== _asbp_joueur OtherActor)
    (`/Game/Characters/BP_Joueur.PickupXP` _asbp_joueur)
    (`self.K2_DestroyActor`)))

(fn `UserConstructionScript`)